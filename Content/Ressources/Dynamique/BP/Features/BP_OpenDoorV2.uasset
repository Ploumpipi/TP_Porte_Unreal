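; Door actor that swings open and closed on its yaw axis, paired with a pressure plate actor (Actionneur).
; COpenDoor's open and close events play and reverse the OuverturePorte timeline, which drives the rotation.
; On plate overlap, PoidsDesActeurs sums the static mesh masses of overlapping actors into PoidsTotal; end overlap zeroes it.
; Nothing in this graph reads that weight to trigger the door.
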(event OnActorBeginOverlap(Actionneur)
  (params (OverlappedActor :type Actor%20Object%20Reference) (OtherActor :type Actor%20Object%20Reference))
  ;[1 1 1] On Begin overlap PressurePlate
  (Variables|Default|SetpoidsTotal 0.0)
  (CallFunction|PoidsDesActeurs OverlappedActor))

(event OnActorEndOverlap(Actionneur)
  (params (OverlappedActor :type Actor%20Object%20Reference) (OtherActor :type Actor%20Object%20Reference))
  ;[1 1 1] On end overlap PressurePlate
  (Variables|Default|SetpoidsTotal 0.0))

(event OpenDoor(COpenDoor)
  (bind _rotationporte (Timeline|OuverturePorte Play)
    (:Update
      (Transformation|SetActorRotation (Math|Rotator|MakeRotator 0.0 0.0 _rotationporte)))))

(event CloseDoor(COpenDoor)
  (bind _rotationporte (Timeline|OuverturePorte Reverse)
    (:Update
      (Transformation|SetActorRotation (Math|Rotator|MakeRotator 0.0 0.0 _rotationporte)))))

(fn ConstructionScript)

(fn PoidsDesActeurs
  (params (Acteur :type Actor%20Object%20Reference))
  (bind _output_get (Variables|Default|SetTableauActeurs (Collision|GetOverlappingActors Acteur "/Script/Engine.Actor" :!class /Script/Engine.Actor)))
  (for _array_element _output_get
    (Variables|Default|SetpoidsTotal (+ (Physics|GetMass (Actor|GetComponentbyClass _array_element "/Script/Engine.StaticMeshComponent")) (Variables|Default|GetpoidsTotal)))))